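; Harpoon projectile that pulls the player toward surfaces tagged "Harpoon" when it hits them.
; On a valid hit it stores the player's location and the hit point as grapple endpoints on Player_BP_WP, then calls MoveHarpoon.
; It polls on a short delay while the player's movement mode is None, then destroys itself; the following Enemy tag check is empty.
; Other hits destroy it immediately and clear the player's IsHarpoon flag.
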(event Collision|EventHit
  (params (MyComp :type Primitive%20Component%20Object%20Reference) (Other :type Actor%20Object%20Reference) (OtherComp :type Primitive%20Component%20Object%20Reference) (bSelfMoved :type Boolean) (HitLocation :type Vector :default "0, 0, 0") (HitNormal :type Vector :default "0, 0, 0") (NormalImpulse :type Vector :default "0, 0, 0") (Hit :type Hit%20Result%20Structure%20%28by%20ref%29))
  ;[1 1 1] Set Harpoon
  (bind _asplayer_bp_wp (Utilities|Casting|CastToPlayer_BP_WP (Game|GetPlayerCharacter 0)))
  (Variables|Default|SetAs%20Player%20BP%20WP _asplayer_bp_wp)
  (if (Actor|ActorHasTag Other "Harpoon")
    (Variables|/Game/Blueprint/1Character/Player_BP_WP.Player_BP_WP_C|SetGrappleStartLoc _asplayer_bp_wp (Transformation|GetActorLocation _asplayer_bp_wp))
    (Variables|/Game/Blueprint/1Character/Player_BP_WP.Player_BP_WP_C|SetGrappleEndLoc _asplayer_bp_wp HitLocation)
    (Default|MoveHarpoon _asplayer_bp_wp)
    (Utilities|FlowControl|Delay 0.1 :!label _label)
    (if (Utilities|Enum|NotEqual(Enum) (Variables|/Script/Engine.CharacterMovementComponent|GetMovementMode (Variables|/Script/Engine.Character|GetCharacterMovement _asplayer_bp_wp)) "MOVE_None")
      (Actor|DestroyActor)
      (if (Actor|ActorHasTag Other "Enemy")
        _)
      (else
        (goto _label)))
    (else
      (Actor|DestroyActor)
      (Variables|/Game/Blueprint/1Character/Player_BP_WP.Player_BP_WP_C|SetIsHarpoon (Variables|Default|GetAs%20Player%20BP%20WP) false))))

(fn ConstructionScript)