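; Shotgun weapon Blueprint that fires a spread of shell projectiles from its Arrow component.
; Shoot Shotgun spawns one scaled-down 3ShotgunShell_BP_WP actor per pellet at the arrow's location.
; Get Spray Angle gives each pellet its own rotation from a random unit vector in a cone around the arrow's forward direction, with MaxSpreadAngle as the half-angle.
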(fn ConstructionScript)

(fn ShootShotgun
  (bind _arrow (Variables|Default|GetArrow))
  (for _index (range 1 (Variables|Default|GetPellets))
    (Game|SpawnActorfromClass "/Game/Blueprint/3Ammo/3ShotgunShell_BP_WP.3ShotgunShell_BP_WP_C" (Math|Transform|MakeTransform (.location (Transformation|GetWorldTransform _arrow)) (CallFunction|GetSprayAngle (Math|Vector|GetForwardVector (Transformation|GetWorldRotation _arrow)) (Variables|Default|GetMax%20Spread%20Angle)) "0.300000,0.300000,0.300000") "Undefined" 0 0)))

(fn GetSprayAngle
  (params (Muzzle%20Direction :type Vector) (Max%20Angle :type Float%20%28double-precision%29))
  (return (Math|Rotator|MakeRotfromX (Math|Random|RandomUnitVectorinConeinDegrees Muzzle%20Direction Max%20Angle))))